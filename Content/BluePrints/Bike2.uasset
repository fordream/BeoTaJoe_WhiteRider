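; Bike2 is a physics-driven bike Blueprint that propels itself every frame without reading player input.
; On BeginPlay it attaches the root component to BodyCollider, keeping world position.
; Tick applies a constant X-axis impulse to BodyCollider and Y-axis angular impulses to both wheels, with no delta-time scaling.
; Actor overlaps spawn an effect at BodyCollider, though no effect asset is specified, and a wheel-torque node is left unwired.
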(event EventBeginPlay
  (Class|Actor|AttachRootComponentto (Variables|Default|GetBodyCollider) "None" "KeepWorldPosition" true))

(event Collision|EventActorBeginOverlap
  (params (OtherActor :type Actor%20Object%20Reference))
  (Class|NiagaraFunctionLibrary|SpawnEffectatLocation 0 (Transformation|GetSocketLocation (Variables|Default|GetBodyCollider) "None") "0.000000, 0, 0" true))

(event EventTick
  (params (DeltaSeconds :type Float%20%28single-precision%29))
  (Physics|AddImpulse (Variables|Default|GetBodyCollider) "1000.000000,0.000000, 0" "None" false)
  (Class|PrimitiveComponent|AddAngularImpulse (Variables|Default|Getwheel2) "0,2000.000000, 0" "None" false)
  (Class|PrimitiveComponent|AddAngularImpulse (Variables|Default|Getwheel1) "0.000000,2000.000000,0.000000" "None" false))

(fn ConstructionScript)