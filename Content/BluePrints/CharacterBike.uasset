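; CharacterBike is a physics-driven bike character that constantly pushes itself along world +X.
; Each Tick applies an impulse to the ChracterNoWheelSprite body until its X velocity reaches a cap, then clamps X while preserving Y and Z.
; The push is applied per frame without delta-time scaling, so acceleration depends on frame rate.
; The construction script calls AttachTo on the Box component; BeginPlay and overlap events are empty.
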(event EventBeginPlay)

(event Collision|EventActorBeginOverlap
  (params (OtherActor :type Actor%20Object%20Reference)))

(event EventTick
  (params (DeltaSeconds :type Float%20%28single-precision%29))
  (bind _returnvalue (Physics|GetPhysicsLinearVelocity (Variables|Default|GetChracterNoWheel_Sprite) "None"))
  (if (>= (.X (Math|Vector|BreakVector _returnvalue)) 7e+02)
    (Class|PrimitiveComponent|SetAllPhysicsLinearVelocity (Variables|Default|GetChracterNoWheel_Sprite) (Math|Vector|MakeVector 7e+02 (.Y (Math|Vector|BreakVector _returnvalue)) (.Z (Math|Vector|BreakVector _returnvalue))) false)
    (else
      (Physics|AddImpulse (Variables|Default|GetChracterNoWheel_Sprite) "1000.000000, 0, 0" "None" false))))

(fn ConstructionScript
  (Class|SceneComponent|Attachto (Variables|Default|GetBox) 0 "None" "KeepRelativeOffset" true))